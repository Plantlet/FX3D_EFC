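; BP_Projectile is a projectile that pushes physics objects when it hits.
; A hit on a simulating component applies a velocity-scaled impulse at the projectile's location, then destroys it.
; Other hits run a multi-sphere trace at the hit point, applying radial and angular impulses to each traced component.
; The radial origin uses the impact normal, and destruction sits inside the loop, so it requires a trace hit.
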(event `self.ReceiveHit`
  (params (MyComp :type "PrimitiveComponent Object Reference") (Other :type "Actor Object Reference") (OtherComp :type "PrimitiveComponent Object Reference") (bSelfMoved :type Boolean) (HitLocation :type "Vector Structure") (HitNormal :type "Vector Structure") (NormalImpulse :type "Vector Structure") (Hit :type "HitResult Structure (by ref)"))
  ;[1 1 1] Checking if there's a direct hit on objects or not
  (set `self.Hit Location` HitLocation)
  (if (`SceneComponent.IsSimulatingPhysics` OtherComp "None")
    (`self.AddImpulse`)
    (else
      (`self.AddRadialForce`))))

(event `AddImpulse`
  ;[1 1 1] Add Impulse
  (`PrimitiveComponent.AddImpulseAtLocation` (stale `self.ReceiveHit` OtherComp) (* (`self.GetVelocity`) 50.0) (`self.K2_GetActorLocation`) "None")
  (`self.K2_DestroyActor`) ; Then destroy this projectile
)

(event `AddRadialForce`
  (bind _hit_location (`self.Hit Location`))
  ;[1 1 1] Add Radial Force
  (bind _outhits (`KismetSystemLibrary.SphereTraceMulti` _hit_location (* _hit_location 1.0) 150.0 "TraceTypeQuery1"))
  (for _array_element _outhits
    (bind (_bblockinghit _binitialoverlap _time _distance _location _impactpoint _normal _impactnormal _physmat _hitactor _hitcomponent) (`GameplayStatics.BreakHitResult` _array_element))
    (`PrimitiveComponent.AddRadialImpulse` _hitcomponent _impactnormal 1000.0 100000.0 "RIF_Constant" false)
    (`PrimitiveComponent.AddAngularImpulseInDegrees` _hitcomponent (* _impactnormal 200.0) "None" true)
    (`self.K2_DestroyActor`)))

(fn `UserConstructionScript`)