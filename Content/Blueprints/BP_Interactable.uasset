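; Interactable actor that levitates, glows and explodes when interacted with, then destroys itself.
; Interact enables physics without gravity and applies an upward impulse plus random spin, while particles and a timeline animate the material threshold and light intensity.
; When the timeline finishes, it spawns a colored explosion and destroys the actor once that system completes.
; The construction script creates the dynamic material and applies one shared Color to material, particles and light.
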(event `/Game/Blueprints/BPi_Interact.Interact`
  (`|ExecutionSequence`
    (:`then_0`
      (`self.Levitate`))
    (:`then_1`
      (`self.Animate`))))

(event `Levitate`
  (bind _staticmesh (`self.StaticMesh`))
  ;[1 1 1] Levitation
  ;;[1 1 1] Simulating On, Gravity off
  (`PrimitiveComponent.SetSimulatePhysics` _staticmesh true)
  (`PrimitiveComponent.SetEnableGravity` _staticmesh false)
  ;;[1 1 1] Impulses
  (`PrimitiveComponent.AddImpulseAtLocation` _staticmesh (0.0 0.0 100000.0) (`SceneComponent.K2_GetComponentLocation` _staticmesh) "None")
  (`PrimitiveComponent.AddAngularImpulseInDegrees` _staticmesh (* (`KismetMathLibrary.RandomUnitVector`) 100.0) "None" true))

(event `Animate`
  (`ActorComponent.Activate` (`self.P_Particles`) false) ; activate the particle system
  (bind (_direction _alpha _lightflickering) (`Timeline|AnimateMaterial`)
    (:`Update`
      ;[1 1 1] Animate the material and light intensity
      (`MaterialInstanceDynamic.SetScalarParameterValue` (`self.DynamicMaterialInstance`) "Threshold" (`KismetMathLibrary.Lerp` 1.0 0.0 _alpha))
      (`LightComponent.SetIntensity` (`self.PointLight`) (`KismetMathLibrary.Lerp` 2000.0 10000.0 _lightflickering)))
    (:`Finished`
      (`self.Explode`) ; Spawn the explosion on finished
    )))

(event `Explode`
  (`ActorComponent.Deactivate` (`self.P_Particles`)) ; Deactivate previous system
  ;[1 1 1] Spawns exploding particles
  (bind _returnvalue (`NiagaraFunctionLibrary.SpawnSystemAtLocation` null (`SceneComponent.K2_GetComponentLocation` (`self.StaticMesh`))))
  (`FXSystemComponent.SetColorParameter` _returnvalue "Color" (`self.Color`))
  ;[1 1 1] When the systems finishes, kill the actor.
  (add `NiagaraComponent.OnSystemFinished` _returnvalue (delegate `OnSystemFinished_Event_0`)))

(event `OnSystemFinished_Event_0`
  (params (PSystem :type "NiagaraComponent Object Reference"))
  ;[1 1 1] When the systems finishes, kill the actor.
  (`self.K2_DestroyActor`))

(fn `UserConstructionScript`
  (bind _staticmesh (`self.StaticMesh`))
  (bind _color (`self.Color`))
  (`/Engine/EditorBlueprintResources/StandardMacros.DoOnce` false
    (:`Completed`
      (bind _returnvalue (`PrimitiveComponent.CreateDynamicMaterialInstance` _staticmesh 0 (`PrimitiveComponent.GetMaterial` _staticmesh 0) "None"))
      (bind _output_get (set `self.DynamicMaterialInstance` _returnvalue))
      ;[1 1 1] Set colors
      (`MaterialInstanceDynamic.SetVectorParameterValue` _output_get "EmissiveColor" _color) ; Set emissive material color
      (`FXSystemComponent.SetColorParameter` (`self.P_Particles`) "Color" _color) ; Set particles color
      (`LightComponent.SetLightColor` (`self.PointLight`) _color true) ; Set light color
    )))