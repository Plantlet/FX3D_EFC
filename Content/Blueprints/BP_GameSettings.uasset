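; BP_GameSettings holds gameplay tuning values for spell charge and tracing, plus a debug print toggle, and hands them to the player character.
; On BeginPlay it sends the charge threshold, trace length, multiple-trace, secondary-spell trace and debug flags to player 0's character through a GetGameSettingsMessage call.
; Its construction script only assigns three of these variables to themselves, so it derives no new values.
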(event `self.ReceiveBeginPlay`
  (message `/Game/Blueprints/BPi_Interact.GetGameSettings` (`GameplayStatics.GetPlayerCharacter` 0) (`self.ChargeThreshold`) (`self.Trace Length`) (`self.TraceMultipleTimes`) (`self.Secondary Spell Trace`) (`self.Show Debug Prints`)))

(fn `UserConstructionScript`
  (set `self.TraceMultipleTimes` (`self.TraceMultipleTimes`))
  (set `self.Secondary Spell Trace` (`self.Secondary Spell Trace`))
  (set `self.ChargeThreshold` (`self.ChargeThreshold`)))